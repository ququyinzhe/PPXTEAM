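; BP_Seagull_GroundToAir is a seagull character Blueprint that starts the level walking on the ground.
; On BeginPlay it randomizes its run-away and fly-away distances and walk speed within min/max ranges, then sets walking movement.
; It then issues a single AI move to a random navigable point around its location.
; The two distances are only stored here; this graph contains no fleeing or takeoff logic.
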(event EventBeginPlay)

(event Collision|EventActorBeginOverlap
  (params (OtherActor :type Actor%20Object%20Reference)))

(event EventTick
  (params (DeltaSeconds :type Float%20%28single-precision%29))
  (|CallParentFunction 0.0))

(event EventBeginPlay
  (bind _self self)
  ;[1 1 1] Start Level walking on the ground
  ;;[1 1 1] Set runAway and FlyAway Distances
  (Variables|Default|SetBirdRunAwayDistance (Math|Random|RandomFloatinRange (Variables|Default|GetRunAwayDistance_Min) (Variables|Default|GetRunAwayDistance_Max)))
  (Variables|Default|SetBirdFlyAwayDistance (Math|Random|RandomFloatinRange (Variables|Default|GetFlyAwayDistance_Min) (Variables|Default|GetFlyAwayDistance_Max)))
  ;;[1 1 1] set movement to Walking
  (Pawn|Components|CharacterMovement|SetMovementMode (Variables|Character|GetCharacterMovement) "MOVE_Walking" 0)
  (Variables|/Script/Engine.CharacterMovementComponent|SetMaxWalkSpeed (Variables|Character|GetCharacterMovement) (Math|Random|RandomFloatinRange (Variables|Default|GetWalkSpeed_Min) (Variables|Default|GetWalkSpeed_Max)))
  (AI|AIMoveTo _self (Class|NavigationSystem|GetRandomPointinNavigableRadius (Transformation|GetActorLocation _self) 2e+03) 0 5e+02 false))

(fn ConstructionScript
  (|CallParentFunction))