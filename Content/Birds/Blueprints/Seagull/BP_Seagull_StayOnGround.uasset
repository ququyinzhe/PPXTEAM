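; Seagull character variant that starts on the ground in walking mode.
; On BeginPlay it randomizes its run-away, fly-away and jump-away distances within min/max ranges, sets CharacterMovement to Walking, updates the walking and flying flags and enables capsule query and physics collision.
; The file only initializes this state and contains no logic that acts on those distances.
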(event EventBeginPlay
  (|CallParentFunction))

(event Collision|EventActorBeginOverlap
  (params (OtherActor :type Actor%20Object%20Reference)))

(event EventTick
  (params (DeltaSeconds :type Float%20%28single-precision%29))
  (|CallParentFunction 0.0))

(event EventBeginPlay
  ;[1 1 1] Stay on the ground
  ;;[1 1 1] Set runAway and FlyAway Distances
  (Variables|Default|SetBirdRunAwayDistance (Math|Random|RandomFloatinRange (Variables|Default|GetRunAwayDistance_Min) (Variables|Default|GetRunAwayDistance_Max)))
  (Variables|Default|SetBirdFlyAwayDistance (Math|Random|RandomFloatinRange (Variables|Default|GetFlyAwayDistance_Min) (Variables|Default|GetFlyAwayDistance_Max)))
  ;;[1 1 1] set movement to Walking
  (Pawn|Components|CharacterMovement|SetMovementMode (Variables|Character|GetCharacterMovement) "MOVE_Walking" 0)
  ;;[1 1 1] Set Is_Walking? and Is_Flying? Bool
  (Variables|Default|SetIs_Flying? false)
  (Variables|Default|SetIs_Walking? true)
  ;;[1 1 1] Enable Collision
  (Collision|SetCollisionEnabled (Variables|Default|GetCapsuleComponent) "QueryAndPhysics")
  ;;[1 1 1] Set Jump Away Distance
  (Variables|Default|SetBirdJumpAwayDistance (Math|Random|RandomFloatinRange (Variables|Default|GetJumpAwayDistance_Min) (Variables|Default|GetJumpAwayDistance_Max))))

(fn ConstructionScript
  (|CallParentFunction))