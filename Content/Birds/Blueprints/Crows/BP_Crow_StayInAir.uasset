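; BP_Crow_StayInAir is a crow variant that stays in flight from the start of play.
; BeginPlay sets character movement to Flying, updates the flying and walking flags, and disables capsule collision.
; It then loops indefinitely, picking a random forward speed between the minimum and maximum fly speeds and re-rolling it after a random delay.
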(event EventBeginPlay
  (|CallParentFunction))

(event EventActorBeginOverlap
  (params (OtherActor :type Actor%20Object%20Reference)))

(event EventTick
  (params (DeltaSeconds :type Float%20%28single-precision%29))
  (|CallParentFunction 0.0))

(event EventBeginPlay
  ;[1 1 1] Fly_Forever
  ;;[1 1 1] set movement to flying
  (Pawn|Components|CharacterMovement|SetMovementMode (Variables|Character|GetCharacterMovement) "MOVE_Flying" 0)
  ;;[1 1 1] Set Is_Walking? and Is_Flying? Bool
  (Variables|Default|SetIs_Flying? true)
  (Variables|Default|SetIs_Walking? false)
  ;;[1 1 1] Disable Collision
  (Collision|SetCollisionEnabled (Variables|Default|GetCapsuleComponent) "NoCollision")
  ;;[1 1 1] Set Fly Speed
  (Variables|Default|SetCurrent%20forward%20speed (Math|Random|RandomFloatinRange (Variables|Default|GetFlySpeed_Min) (Variables|Default|GetFlySpeed_Max)) :!label _label)
  ;;[1 1 1] Change FlySpeed every now and then
  (Utilities|FlowControl|Delay (Math|Random|RandomFloatinRange 3e+01 6e+01))
  (goto _label))

(fn ConstructionScript
  (|CallParentFunction))