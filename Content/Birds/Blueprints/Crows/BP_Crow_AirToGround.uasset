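; BP_Crow_AirToGround is a crow variant that starts the level already airborne, with no take-off, and later becomes due to land on the ground.
; On BeginPlay it randomizes run-away and fly-away distances and forward speed within min/max ranges and sets movement to Flying.
; After a random flight-time delay it raises TimeToLand; the landing behavior itself is not in these graphs.
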(event EventBeginPlay
  (|CallParentFunction))

(event EventActorBeginOverlap
  (params (OtherActor :type Actor%20Object%20Reference)))

(event EventTick
  (params (DeltaSeconds :type Float%20%28single-precision%29))
  (|CallParentFunction 0.0))

(event EventBeginPlay
  ;[1 1 1] Start out Flying without TakeOff
  ; Set how long to fly before landing on the ground at the begining of the level
  ;;[1 1 1] Set runAway and FlyAway Distances
  (Variables|Default|SetBirdRunAwayDistance (Math|Random|RandomFloatinRange (Variables|Default|GetRunAwayDistance_Min) (Variables|Default|GetRunAwayDistance_Max)))
  (Variables|Default|SetBirdFlyAwayDistance (Math|Random|RandomFloatinRange (Variables|Default|GetFlyAwayDistance_Min) (Variables|Default|GetFlyAwayDistance_Max)))
  ;;[1 1 1] set movement to flying
  (Pawn|Components|CharacterMovement|SetMovementMode (Variables|Character|GetCharacterMovement) "MOVE_Flying" 0)
  ;;[1 1 1] Set Fly Speed
  (Variables|Default|SetCurrent%20forward%20speed (Math|Random|RandomFloatinRange (Variables|Default|GetFlySpeed_Min) (Variables|Default|GetFlySpeed_Max)))
  ;;[1 1 1] Set How long to fly before its time to land
  (Utilities|FlowControl|Delay (Math|Random|RandomFloatinRange (Variables|Default|GetFlyTime_Min) (Variables|Default|GetFlyTime_Max)))
  ;;[1 1 1] Set TimeToLand to True
  (Variables|Default|SetTimeToLand true))

(fn ConstructionScript
  (|CallParentFunction))