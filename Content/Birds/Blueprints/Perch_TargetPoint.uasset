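; Perch target point that lets one flying bird NPC land, rest and take off again.
; On sphere overlap, an occupied perch sends the bird away, while a free one claims a bird that is looking for a perch and stops its movement.
; A timeline lerps the bird to the FaceThisWay arrow, optionally matching its yaw.
; After a random perch delay, the bird flies away and the perch frees up.
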(event OnComponentBeginOverlap(Sphere)
  (params (OtherActor :type Actor%20Object%20Reference) (OtherComp :type Primitive%20Component%20Object%20Reference) (OtherBodyIndex :type Integer) (bFromSweep :type Boolean) (SweepResult :type Hit%20Result%20Structure%20%28by%20ref%29))
  (bind _facethisway (Variables|Default|GetFaceThisWay))
  (bind _returnvalue (Transformation|GetWorldRotation _facethisway))
  (bind (_roll _pitch) (Math|Rotator|BreakRotator _returnvalue))
  ;[1 1 1] Is the Perch Occupied?
  (if (Variables|Default|GetOccupied?)
    ;[1 1 1] Tell bird to fly away if perch is occupied
    (bind _asbp_npc_perching_flying_bird_base (Utilities|Casting|CastToBP_NPC_PerchingFlying_Bird_Base OtherActor))
    (Variables|/Game/Birds/Blueprints/Base_Classes/BP_NPC_PerchingFlying_Bird_Base.BP_NPC_PerchingFlying_Bird_Base_C|SetIsLookingForPerch? _asbp_npc_perching_flying_bird_base false)
    (Variables|/Game/Birds/Blueprints/Base_Classes/BP_NPC_PerchingFlying_Bird_Base.BP_NPC_PerchingFlying_Bird_Base_C|SetFlyAway? _asbp_npc_perching_flying_bird_base true)
    (else
      ;[1 1 1] Is the bird looking for a perch?
      (bind _asbp_npc_perching_flying_bird_base_2 (Utilities|Casting|CastToBP_NPC_PerchingFlying_Bird_Base OtherActor))
      (if (Variables|/Game/Birds/Blueprints/Base_Classes/BP_NPC_PerchingFlying_Bird_Base.BP_NPC_PerchingFlying_Bird_Base_C|GetIsLookingForPerch? _asbp_npc_perching_flying_bird_base_2)
        ;[1 1 1] Tell bird to stop moving
        (Components|Movement|StopMovementImmediately (Variables|/Script/Engine.Character|GetCharacterMovement _asbp_npc_perching_flying_bird_base_2))
        (Variables|/Game/Birds/Blueprints/Base_Classes/BP_NPC_PerchingFlying_Bird_Base.BP_NPC_PerchingFlying_Bird_Base_C|SetCurrent%20forward%20speed _asbp_npc_perching_flying_bird_base_2 0.0)
        ;[1 1 1] Set the perch to occupied
        (Variables|Default|SetOccupied? true)
        ;[1 1 1] Fly to perch
        (Variables|/Game/Birds/Blueprints/Base_Classes/BP_NPC_PerchingFlying_Bird_Base.BP_NPC_PerchingFlying_Bird_Base_C|SetFlyToPerch? _asbp_npc_perching_flying_bird_base_2 true)
        (Variables|/Game/Birds/Blueprints/Base_Classes/BP_NPC_PerchingFlying_Bird_Base.BP_NPC_PerchingFlying_Bird_Base_C|SetIs_Flying? _asbp_npc_perching_flying_bird_base_2 false)
        (Variables|/Game/Birds/Blueprints/Base_Classes/BP_NPC_PerchingFlying_Bird_Base.BP_NPC_PerchingFlying_Bird_Base_C|SetIsLookingForPerch? _asbp_npc_perching_flying_bird_base_2 false)
        (Variables|Default|SetFlyFromHere_Perching (Transformation|GetActorLocation _asbp_npc_perching_flying_bird_base_2))
        (Variables|Default|SetFlyToHere_Perching (Transformation|GetWorldLocation (Variables|Default|GetFaceThisWay)))
        (Variables|Default|SetCurrentRotation (Transformation|GetActorRotation _asbp_npc_perching_flying_bird_base_2))
        (if (Variables|Default|GetUseFaceThisWayArrow?)
          (Variables|Default|SetDesiredRotation (Transformation|GetWorldRotation (Variables|Default|GetFaceThisWay)))
          (else
            (Variables|Default|SetDesiredRotation (Math|Rotator|MakeRotator _roll _pitch (.Yaw (Math|Rotator|BreakRotator (Transformation|GetActorRotation _asbp_npc_perching_flying_bird_base_2)))))))
        (Components|Timeline|SetPlayRate (Variables|Default|GetFlyToPerch) (Variables|Default|GetFlyToPerch_Speed))
        (bind _newtrack_1 (Timeline|FlyToPerch PlayFromStart)
          (:Update
            (Transformation|SetActorLocation _asbp_npc_perching_flying_bird_base_2 (Math|Vector|Lerp(Vector) (Variables|Default|GetFlyFromHere_Perching) (Variables|Default|GetFlyToHere_Perching) _newtrack_1) false false)
            (Transformation|SetActorRotation _asbp_npc_perching_flying_bird_base_2 (Math|Rotator|Lerp(Rotator) (Variables|Default|GetCurrentRotation) (Variables|Default|GetDesiredRotation) _newtrack_1)))
          (:Finished
            ;[1 1 1] Tell bird to perch
            (Variables|/Game/Birds/Blueprints/Base_Classes/BP_NPC_PerchingFlying_Bird_Base.BP_NPC_PerchingFlying_Bird_Base_C|SetFlyToPerch? _asbp_npc_perching_flying_bird_base_2 false)
            (Variables|/Game/Birds/Blueprints/Base_Classes/BP_NPC_PerchingFlying_Bird_Base.BP_NPC_PerchingFlying_Bird_Base_C|SetIsPerched? _asbp_npc_perching_flying_bird_base_2 true)
            ;[1 1 1] Set how long to perch
            (Utilities|FlowControl|Delay (Math|Random|RandomFloatinRange 5.0 5e+01))
            ;[1 1 1] Tell Bird to Fly Away
            (Variables|/Game/Birds/Blueprints/Base_Classes/BP_NPC_PerchingFlying_Bird_Base.BP_NPC_PerchingFlying_Bird_Base_C|SetFlyAway? _asbp_npc_perching_flying_bird_base_2 true)
            (Variables|/Game/Birds/Blueprints/Base_Classes/BP_NPC_PerchingFlying_Bird_Base.BP_NPC_PerchingFlying_Bird_Base_C|SetAllPerchesAreFull _asbp_npc_perching_flying_bird_base_2 false)
            ;[1 1 1] Set the perch to not occupied
            (Variables|Default|SetOccupied? false)))))))

(fn ConstructionScript)